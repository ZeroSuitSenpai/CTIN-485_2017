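; BasicEnemy is an enemy Blueprint that chases the player pawn and dies when bullets deplete its Health.
; Tick repeatedly calls MoveComponentTo on the root component, targeting the player pawn's current location.
; Overlapping a "BulletTag" actor destroys it, flashes the Body material and subtracts Health, then either destroys the enemy or restores the material after a short delay.
; Damage is handled inline in the overlap event; the TakeDamage function is empty.
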(event EventBeginPlay)

(event Collision|EventActorBeginOverlap
  (params (OtherActor :type Actor%20Object%20Reference))
  (if (Actor|ActorHasTag OtherActor "BulletTag")
    (Actor|DestroyActor OtherActor)
    (Rendering|Material|SetMaterial (Variables|Default|GetBody) 0 "/Game/StarterContent/Materials/HitFlash.HitFlash")
    (Variables|Default|SetHealth (- (Variables|Default|GetHealth) 1.0))
    (if (<= (Variables|Default|GetHealth) 0.0)
      (Actor|DestroyActor)
      (else
        (Utilities|FlowControl|Delay 0.2)
        (Rendering|Material|SetMaterial (Variables|Default|GetBody) 0 "/Game/StarterContent/Materials/M_Brick_Clay_New.M_Brick_Clay_New")
        (Development|PrintString "Enemy was hit")))))

(event EventTick
  (params (DeltaSeconds :type Float%20%28single-precision%29))
  (Components|MoveComponentTo (Variables|Transformation|GetRootComponent) (Transformation|GetActorLocation (Game|Player|GetPlayerPawn 0)) "0, 0, 0" false false 0.3 false))

(fn ConstructionScript)

(fn TakeDamage)
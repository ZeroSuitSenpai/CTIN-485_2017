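; RotationController is a player controller that drives a pawn with top-down movement, mouse aiming and shooting.
; MoveUp and MoveRight axes move the pawn along fixed world X and Y.
; Each tick it yaws the pawn toward the deprojected mouse world position, without any trace, and locks control rotation straight down.
; FireBullet casts the pawn to RotationCharacter and calls FireProjectile, printing a message if the cast fails.
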(event EventBeginPlay)

(event EventTick
  (params (DeltaSeconds :type Float%20%28single-precision%29))
  (bind _returnvalue (Pawn|GetControlledPawn))
  ;[1 1 1] MouseRotation
  (Transformation|SetActorRotation _returnvalue (Math|Rotator|MakeRotator 0.0 0.0 (.Yaw (Math|Rotator|BreakRotator (Math|Rotator|FindLookatRotation (Transformation|GetActorLocation _returnvalue) (.WorldLocation (Game|Player|ConvertMouseLocationToWorldSpace)))))))
  (Pawn|SetControlRotation (Math|Rotator|MakeRotator 0.0 -9e+01 0.0)))

(event Input|ActionEvents|InputActionFireBullet
  (params (Key :type Key%20Structure))
  (:Pressed
    (bind _asrotation_character (Utilities|Casting|CastToRotationCharacter (Pawn|GetControlledPawn))
      (:then
        (Default|FireProjectile _asrotation_character))
      (:CastFailed
        (Development|PrintString "Character cast FAILED!")))))

(event Input|AxisEvents|InputAxisMoveUp
  (params (AxisValue :type Float%20%28single-precision%29))
  ;[1 1 1] Keyboard Movement
  (Pawn|Input|AddMovementInput (Pawn|GetControlledPawn) "1.000000, 0, 0" AxisValue false))

(event Input|AxisEvents|InputAxisMoveRight
  (params (AxisValue :type Float%20%28single-precision%29))
  ;[1 1 1] Keyboard Movement
  (Pawn|Input|AddMovementInput (Pawn|GetControlledPawn) "0,1.000000, 0" AxisValue false))

(fn ConstructionScript)
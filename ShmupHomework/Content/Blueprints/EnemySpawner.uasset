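; Spawner actor that periodically creates an enemy at its own transform, choosing at random between BasicEnemy and WarpEnemy.
; A frame-counted Timer starts at a random offset on BeginPlay, increments each Tick, and resets after triggering a spawn at a fixed threshold, so the interval depends on frame rate.
; SpawnEnemy and SpawnWarper each spawn their class with its own starting Health.
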(event EventBeginPlay
  (Variables|Default|SetTimer (Math|Conversions|ToFloat(Integer) (Math|Random|RandomIntegerinRange 0 500))))

(event Collision|EventActorBeginOverlap
  (params (OtherActor :type Actor%20Object%20Reference)))

(event EventTick
  (params (DeltaSeconds :type Float%20%28single-precision%29))
  (Variables|Default|SetTimer (+ (Variables|Default|GetTimer) 1.0))
  (if (>= (Variables|Default|GetTimer) 1e+03)
    (if (== (Math|Random|RandomIntegerinRange 0 1) 0)
      (CallFunction|SpawnEnemy)
      (else
        (CallFunction|SpawnWarper)))
    (Variables|Default|SetTimer 0.0)))

(fn ConstructionScript)

(fn SpawnEnemy
  (Game|SpawnActorfromClass "/Game/Blueprints/BasicEnemy.BasicEnemy_C" (Transformation|GetActorTransform) "Undefined" 0 3.0 0))

(fn SpawnWarper
  (Game|SpawnActorfromClass "/Game/Blueprints/WarpEnemy.WarpEnemy_C" (Transformation|GetActorTransform) "Undefined" 0 2.0 0))
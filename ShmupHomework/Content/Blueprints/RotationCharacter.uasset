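; RotationCharacter is a Blueprint actor with health that takes damage from enemies and can fire bullets.
; It resets Health on BeginPlay, then each overlap with an "Enemy"-tagged actor prints a debug string, deducts a point and destroys the character at zero.
; FireProjectile spawns a non-uniformly scaled Bullet just ahead along the actor's forward vector, though nothing in this file calls it.
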(event EventBeginPlay
  (Variables|Default|SetHealth 1e+01))

(event Collision|EventActorBeginOverlap
  (params (OtherActor :type Actor%20Object%20Reference))
  (if (Actor|ActorHasTag OtherActor "Enemy")
    (Development|PrintString "Hello")
    (Variables|Default|SetHealth (- (Variables|Default|GetHealth) 1.0))
    (if (<= (Variables|Default|GetHealth) 0.0)
      (Actor|DestroyActor))))

(event EventTick
  (params (DeltaSeconds :type Float%20%28single-precision%29)))

(fn ConstructionScript)

(fn FireProjectile
  (bind _returnvalue (Transformation|GetActorRotation))
  (Game|SpawnActorfromClass "/Game/Blueprints/Bullet.Bullet_C" (Math|Transform|MakeTransform (+ (* (Math|Vector|GetForwardVector _returnvalue) 3e+01) (Transformation|GetActorLocation)) _returnvalue "0.500000,0.500000,2.000000") "Undefined" 0 0))
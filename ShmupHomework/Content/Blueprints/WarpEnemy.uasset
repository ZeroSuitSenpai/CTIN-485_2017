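; WarpEnemy is an enemy actor that loses health when hit by bullets and is destroyed at zero.
; Overlapping a BulletTag actor destroys it, removes one health and briefly swaps the Body material to a hit flash.
; Each Tick moves the root to the player-minus-enemy offset, used as a target location, with a negative duration derived from distance.
; The TakeDamage function is an empty stub.
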(event EventBeginPlay)

(event Collision|EventActorBeginOverlap
  (params (OtherActor :type Actor%20Object%20Reference))
  (if (Actor|ActorHasTag OtherActor "BulletTag")
    (Actor|DestroyActor OtherActor)
    (Rendering|Material|SetMaterial (Variables|Default|GetBody) 0 "/Game/StarterContent/Materials/HitFlash.HitFlash")
    (Variables|Default|SetHealth (- (Variables|Default|GetHealth) 1.0))
    (if (<= (Variables|Default|GetHealth) 0.0)
      (Actor|DestroyActor)
      (else
        (Utilities|FlowControl|Delay 0.2)
        (Rendering|Material|SetMaterial (Variables|Default|GetBody) 0 "/Game/StarterContent/Materials/M_Brick_Clay_New.M_Brick_Clay_New")
        (Development|PrintString "Enemy was hit")))))

(event EventTick
  (params (DeltaSeconds :type Float%20%28single-precision%29))
  (bind _returnvalue (Transformation|GetActorLocation))
  (bind _returnvalue_2 (Game|Player|GetPlayerPawn 0))
  (bind _returnvalue_3 (Transformation|GetActorLocation _returnvalue_2))
  (bind _returnvalue_4 (- _returnvalue_3 _returnvalue))
  (Components|MoveComponentTo (Variables|Transformation|GetRootComponent) _returnvalue_4 "0, 0, 0" false false (/ (Math|Vector|VectorLength _returnvalue_4) (- 0.0 1e+02)) false))

(fn ConstructionScript)

(fn TakeDamage)